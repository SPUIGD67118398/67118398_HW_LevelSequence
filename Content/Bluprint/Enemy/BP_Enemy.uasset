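; BP_Enemy is an enemy actor with health, an overhead-style health widget and an alert indicator.
; It initializes its health component on BeginPlay, then handles that component's update event to set the WBP_EnemyHealth percentage and destroy itself at zero health.
; ShowAlert passes a show flag to the same widget to toggle the alert, with no caller inside this Blueprint.
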(event `self.ReceiveBeginPlay`
  (`/Game/Bluprint/Component/BPC_HealthComponent.Inithealth` (`self.BPC_HealthComponent`) 50.0))

(event `self.BPC_HealthComponent.OnUpdateHealth`
  (params (NewHealth :type "Float (double-precision)"))
  (bind _maxhealth (`/Game/Bluprint/Component/BPC_HealthComponent.GetMaxHealth` (`self.BPC_HealthComponent`)))
  (bind _aswbp_enemy_health (cast `/Game/Bluprint/Enemy/WBP_EnemyHealth` (`WidgetComponent.GetWidget` (`self.HealthWidget`))))
  (`/Game/Bluprint/Enemy/WBP_EnemyHealth.SetHealthPercent` _aswbp_enemy_health (/ NewHealth _maxhealth))
  (if (<= NewHealth 0.0)
    (`self.K2_DestroyActor`)))

(fn `ShowAlert`
  (params (Show :type Boolean))
  (bind _aswbp_enemy_health (cast `/Game/Bluprint/Enemy/WBP_EnemyHealth` (`WidgetComponent.GetWidget` (`self.HealthWidget`))))
  (`/Game/Bluprint/Enemy/WBP_EnemyHealth.SetAlert` _aswbp_enemy_health Show))

(fn `UserConstructionScript`)