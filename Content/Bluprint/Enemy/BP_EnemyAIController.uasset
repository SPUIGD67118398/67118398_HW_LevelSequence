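; AI controller for enemy pawns that reacts when its perception detects or loses a target.
; When a player character is sensed, it sets that actor as the controlled BP_Enemy's target and turns on the enemy's alert.
; Any lost stimulus clears the target and hides the alert, without checking whether the lost actor is the player.
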(event `self.AIPerception.OnTargetPerceptionUpdated`
  (params (Actor :type "Actor Object Reference") (Stimulus :type "AIStimulus Structure"))
  (if (`.bSuccessfullySensed` (break `AIStimulus` Stimulus))
    (cast `/Game/Bluprint/ThirdPerson/Blueprints/BP_Player_Character` Actor)
    (bind _asbp_enemy (cast `/Game/Bluprint/Enemy/BP_Enemy` (`self.K2_GetPawn`)))
    (set `/Game/Bluprint/Enemy/BP_Enemy.TargetActor` Actor _asbp_enemy)
    (`/Game/Bluprint/Enemy/BP_Enemy.ShowAlert` _asbp_enemy true)
    (else
      (bind _asbp_enemy_2 (cast `/Game/Bluprint/Enemy/BP_Enemy` (`self.K2_GetPawn`)))
      (set `/Game/Bluprint/Enemy/BP_Enemy.TargetActor` null _asbp_enemy_2)
      (`/Game/Bluprint/Enemy/BP_Enemy.ShowAlert` _asbp_enemy_2 false))))

(fn `UserConstructionScript`)